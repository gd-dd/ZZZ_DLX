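; Blueprint for the Anby playable agent, extending a parent character with walk and idle switching and camera zoom.
; MoveStart and MoveEnd call the parent, then switch the StateMachine between Anby_Walk and Anby_Idle.
; BeginPlay caches the ABP_Anby anim instance and sets the run-start delay, while the mouse wheel adjusts spring arm length.
; Older timed-run, turn-back and turning-tilt logic remains disconnected, leaving Tick empty.
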(event EventBeginPlay
  ;[0.15 0.15 0.15 0.5] BeginPlay
  (|CallParentFunction)
  (bind _asabp_anby (Utilities|Casting|CastToABP_Anby (Components|SkeletalMesh|GetAnimInstance (Variables|Character|GetMesh))))
  (Variables|Default|SetCharacterAnimationBP _asabp_anby)
  (Variables|Default|SetRunStartDuration 3.0))

(event EventTick
  (params (DeltaSeconds :type Float%20%28single-precision%29))
  ;[0.15 0.15 0.15 0.5] Turn and Run
)

(event Input|MouseEvents|MouseWheelAxis
  (params (AxisValue :type Float%20%28single-precision%29))
  ;[0.15 0.15 0.15 0.5] Mouse_Wheel
  (Variables|/Script/Engine.SpringArmComponent|SetTargetArmLength (Variables|Default|GetSpringArm) (+ (Variables|/Script/Engine.SpringArmComponent|GetTargetArmLength (Variables|Default|GetSpringArm)) (* AxisValue -8.0))))

(fn ConstructionScript
  (|CallParentFunction))

(fn MoveStart
  (|CallParentFunction)
  (Default|ChangeState (Variables|Default|GetStateMachine) "Anby_Walk" false))

(fn MoveEnd
  (|CallParentFunction)
  (Default|ChangeState (Variables|Default|GetStateMachine) "Anby_Idle" false)
  (Variables|Default|SetShouldExecuteCheckRunTimer false))