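; Playable MingYing character with camera-relative movement and an orbiting, zoomable spring-arm camera.
; Move turns the mesh to the input direction plus camera yaw, sets the walk flag on ABP_MingYing, and adds movement along the mesh's right vector.
; Camera_rot rotates the spring arm and clamps pitch to CameraRotMax, reapplying yaw with a half-turn offset.
; The mouse wheel adjusts arm length, and debug prints show rotation values.
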(event Custom|Camera_rot
  (params (Camera_rot :type Vector%202D%20Structure))
  (bind (_x _y) (Math|Vector2D|BreakVector2D Camera_rot))
  (bind _springarm (Variables|Default|GetSpringArm))
  (bind _returnvalue (Class|SpringArmComponent|GetTargetRotation _springarm))
  (Development|PrintString (Utilities|String|ToString(Vector2d) Camera_rot))
  (Transformation|AddRelativeRotation (Variables|Default|GetSpringArm) (Math|Rotator|MakeRotator 0.0 (/ _y 1.0) (/ _x 1.0)) false false)
  (Variables|Default|SetSpringArm_Yaw (+ (.yaw _returnvalue) 1.8e+02))
  (if (< (.pitch _returnvalue) (* (Variables|Default|GetCamera%20Rot%20Max) -1.0))
    (Transformation|SetRelativeRotation (Variables|Default|GetSpringArm) (Math|Rotator|MakeRotator 0.0 (* (Variables|Default|GetCamera%20Rot%20Max) -1.0) (Variables|Default|GetSpringArm_Yaw)) false false)
    (elif (> (.pitch _returnvalue) (Variables|Default|GetCamera%20Rot%20Max))
      (Transformation|SetRelativeRotation (Variables|Default|GetSpringArm) (Math|Rotator|MakeRotator 0.0 (Variables|Default|GetCamera%20Rot%20Max) (Variables|Default|GetSpringArm_Yaw)) false false))))

(event Custom|Move
  (params (rotat :type Vector%202D%20Structure) (Is_Press :type Boolean))
  (bind _returnvalue (Math|Conversions|ToVector(Vector2D) rotat))
  (bind _springarm (Variables|Default|GetSpringArm))
  (bind _returnvalue_2 (Class|SpringArmComponent|GetTargetRotation _springarm))
  (bind _yaw (Math|Vector|GetYawPitchfromVector _returnvalue))
  (bind _returnvalue_3 (+ _yaw (.yaw _returnvalue_2)))
  (bind _returnvalue_4 (Math|Rotator|MakeRotator 0.0 0.0 _returnvalue_3))
  (Development|PrintString (Utilities|String|ToString(Rotator) _returnvalue_4))
  (bind _asabp_ming_ying (Utilities|Casting|CastToABP_MingYing (Components|SkeletalMesh|GetAnimInstance (Variables|Character|GetMesh))))
  (if Is_Press
    (Transformation|SetRelativeRotation (Variables|Character|GetMesh) _returnvalue_4 false false))
  (if Is_Press
    (Variables|/Game/BP/Agent/MingYing/ABP_MingYing.ABP_MingYing_C|SetIsWalk _asabp_ming_ying true)
    (else
      (Variables|/Game/BP/Agent/MingYing/ABP_MingYing.ABP_MingYing_C|SetIsWalk _asabp_ming_ying false)))
  (Pawn|Input|AddMovementInput (Math|Vector|GetRightVector (Variables|Character|GetMesh)) 0.15 false))

(event EventBeginPlay
  (Variables|Default|SetCamera%20Rot%20Max 8e+01))

(event Input|MouseEvents|MouseWheelAxis
  (params (AxisValue :type Float%20%28single-precision%29))
  (bind _springarm (Variables|Default|GetSpringArm))
  (Variables|/Script/Engine.SpringArmComponent|SetTargetArmLength _springarm (+ (Variables|/Script/Engine.SpringArmComponent|GetTargetArmLength _springarm) (* AxisValue -8.0))))

(fn ConstructionScript
  (|CallParentFunction))