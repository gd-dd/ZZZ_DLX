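; Player controller for ZZZ combat that turns Enhanced Input into movement, camera, attack and evade commands for the possessed BP_ZZZAgent.
; Move input becomes a camera-relative yaw offset from the actor's rotation, stored on the agent alongside start/end calls.
; The agent's SMAgent receives state and attack invocations, with normal attack also recorded in the GameInstance's InputCacheSystem.
; It also creates an on-screen debug frame and exposes events to add and update its entries.
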(event Custom|AddDebugObject
  (params (Id :type String) (InitText :type String))
  (bind _wb_debugframe (Variables|Default|GetWB_DebugFrame))
  (bind _returnvalue (UserInterface|CreateWidget "/Game/BP/UI/DebugWidget/WB_DebugUnit.WB_DebugUnit_C"))
  (Utilities|IsValid _wb_debugframe
    (:Is%20Valid
      (Default|AddDebugObject _wb_debugframe _returnvalue Id)
      (Default|UpdateDebugObjectText _wb_debugframe Id InitText))))

(event Custom|UpdateDebugObject
  (params (Id :type String) (NewParam :type String))
  (Default|UpdateDebugObjectText (Variables|Default|GetWB_DebugFrame) Id NewParam))

(event Input|EnhancedActionEvents|EnhancedInputActionIA_ZZZ_Move
  (params (ActionValue :type Vector%202D%20Structure) (ElapsedSeconds :type Float%20%28double-precision%29) (TriggeredSeconds :type Float%20%28double-precision%29) (InputAction :type Input%20Action%20Object%20Reference :default "/Game/BP/Input/InputActions/IA_ZZZ_Move.IA_ZZZ_Move"))
  (bind (_x _y) (Math|Vector2D|BreakVector2D ActionValue))
  (bind _currentcharacter (Variables|Default|GetCurrentCharacter))
  (bind _currentcharacter_2 (Variables|Default|GetCurrentCharacter))
  (bind _currentcharacter_3 (Variables|Default|GetCurrentCharacter))
  (bind _currentcharacter_4 (Variables|Default|GetCurrentCharacter))
  (bind _returnvalue (* _x -1.0))
  (bind _camera (Variables|/Game/BP/Agent/BP_ZZZAgent.BP_ZZZAgent_C|GetCamera _currentcharacter))
  (bind _returnvalue_2 (Math|Vector|GetForwardVector _camera))
  (bind _returnvalue_3 (Math|Vector|GetRightVector _camera))
  (bind _returnvalue_4 (* _returnvalue_2 _y))
  (bind _returnvalue_5 (* _returnvalue_3 _returnvalue))
  (bind _returnvalue_6 (+ _returnvalue_4 _returnvalue_5))
  (bind (_x_2 _y_2) (Math|Vector|BreakVector _returnvalue_6))
  (:Triggered
    (Utilities|IsValid _currentcharacter
      (:Is%20Valid
        ;[0.15 0.15 0.15 0.5] Move
        ;;[0.15 0.15 0.15 0.5] Calculate relative rotator
        (bind _output_get (Variables|Default|SetdesiredDirection (Math|Vector|Normalize (Math|Vector|MakeVector _x_2 _y_2 0.0))))
        (bind _output_get_2 (Variables|/Game/BP/Agent/BP_ZZZAgent.BP_ZZZAgent_C|SetCharacterCurrentRotator (Variables|Default|GetCurrentCharacter) (Math|Rotator|MakeRotator 0.0 0.0 (.Yaw (Math|Rotator|BreakRotator (Class|KismetMathLibrary|QuatRotator (* (Math|Conversions|ToQuaternion(Rotator) _output_get) (Class|KismetMathLibrary|QuatInversed (Math|Conversions|ToQuaternion(Rotator) (Transformation|GetActorRotation _currentcharacter))))))))))
        (Development|PrintString (Utilities|String|ToString(Rotator) _output_get_2))
        (Default|StateReinvoke (Variables|/Game/BP/Agent/BP_ZZZAgent.BP_ZZZAgent_C|GetSMAgent (Variables|Default|GetCurrentCharacter)) "ReturnToIdleOrWalk"))))
  (:Started
    (Utilities|IsValid _currentcharacter_4
      (:Is%20Valid
        (Variables|/Game/BP/Agent/BP_ZZZAgent.BP_ZZZAgent_C|SetIsPressMoveButtom _currentcharacter_4 true)
        (Default|MoveStart _currentcharacter_4))))
  (:Completed
    (Utilities|IsValid _currentcharacter_2
      (:Is%20Valid
        (Variables|/Game/BP/Agent/BP_ZZZAgent.BP_ZZZAgent_C|SetIsPressMoveButtom _currentcharacter_2 false)
        ;[0.15 0.15 0.15 0.5] MoveEnd
        (Variables|/Game/BP/Agent/BP_ZZZAgent.BP_ZZZAgent_C|SetCharacterCurrentRotator _currentcharacter_3 "0, 0, 0")
        (Default|MoveEnd _currentcharacter_3)))))

(event Input|EnhancedActionEvents|EnhancedInputActionIA_ZZZ_Camera
  (params (ActionValue :type Vector%202D%20Structure) (ElapsedSeconds :type Float%20%28double-precision%29) (TriggeredSeconds :type Float%20%28double-precision%29) (InputAction :type Input%20Action%20Object%20Reference :default "/Game/BP/Input/InputActions/IA_ZZZ_Camera.IA_ZZZ_Camera"))
  (bind (_x _y) (Math|Vector2D|BreakVector2D ActionValue))
  (Class|PlayerController|AddYawInput _x)
  (Class|PlayerController|AddPitchInput (* _y -1.0)))

(event Input|EnhancedActionEvents|EnhancedInputActionIA_NormalAttack_Press
  (params (ActionValue :type Boolean) (ElapsedSeconds :type Float%20%28double-precision%29) (TriggeredSeconds :type Float%20%28double-precision%29) (InputAction :type Input%20Action%20Object%20Reference :default "/Game/BP/Input/InputActions/IA_NormalAttack_Press.IA_NormalAttack_Press"))
  (bind _currentcharacter (Variables|Default|GetCurrentCharacter))
  (bind _asbp_zzzgame_instance (Utilities|Casting|CastToBP_ZZZGameInstance (Game|GetGameInstance)))
  (Default|AddInputCache (Variables|/Game/BP/Basic/BP_ZZZGameInstance.BP_ZZZGameInstance_C|GetInputCacheSystem _asbp_zzzgame_instance) "NewEnumerator0")
  (Utilities|IsValid _currentcharacter
    (:Is%20Valid
      (Default|AttackInvoke (Variables|/Game/BP/Agent/BP_ZZZAgent.BP_ZZZAgent_C|GetSMAgent _currentcharacter) "NewEnumerator0")
      (Default|StateReinvoke (Variables|/Game/BP/Agent/BP_ZZZAgent.BP_ZZZAgent_C|GetSMAgent (Variables|Default|GetCurrentCharacter)) "NormalAttack"))))

(event Input|EnhancedActionEvents|EnhancedInputActionIA_ZZZ_Evade
  (params (ActionValue :type Boolean) (ElapsedSeconds :type Float%20%28double-precision%29) (TriggeredSeconds :type Float%20%28double-precision%29) (InputAction :type Input%20Action%20Object%20Reference :default "/Game/BP/Input/InputActions/IA_ZZZ_Evade.IA_ZZZ_Evade"))
  (bind _currentcharacter (Variables|Default|GetCurrentCharacter))
  (Utilities|IsValid _currentcharacter
    (:Is%20Valid
      (Default|AttackInvoke (Variables|/Game/BP/Agent/BP_ZZZAgent.BP_ZZZAgent_C|GetSMAgent _currentcharacter) "NewEnumerator5"))))

(event EventBeginPlay
  (Input|AddMappingContext (PlayerController|LocalPlayerSubsystems|GetEnhancedInputLocalPlayerSubsystem self) "/Game/BP/Input/IMC_ZZZCombat.IMC_ZZZCombat" 0 "(bIgnoreAllPressedKeysUntilRelease=True,bForceImmediately=False,bNotifyUserSettings=False)")
  (bind _returnvalue (UserInterface|CreateWidget "/Game/BP/UI/DebugWidget/WB_DebugFrame.WB_DebugFrame_C" self))
  (bind _output_get (Variables|Default|SetWB_DebugFrame _returnvalue))
  (UserInterface|Viewport|AddtoViewport _output_get 0))

(event EventTick
  (params (DeltaSeconds :type Float%20%28single-precision%29)))

(event EventPossess
  (params (PossessedPawn :type Pawn%20Object%20Reference))
  (bind _asbp_zzzagent (Utilities|Casting|CastToBP_ZZZAgent PossessedPawn))
  (Variables|Default|SetCurrentCharacter _asbp_zzzagent))

(fn ConstructionScript)