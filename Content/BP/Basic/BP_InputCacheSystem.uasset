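; BP_InputCacheSystem keeps a short history of recent inputs for other code to query.
; While caching is enabled, new inputs are appended to a capped array, dropping the oldest entry when it is full.
; Reads return the newest entry without removing it, or a fixed fallback enum value when the history is empty, and a cleanup function clears the whole cache.
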(fn AddInputCache
  (params (NewInput :type Enum_ZZZAgentInputType%20Enum :default "NewEnumerator0"))
  (if (Variables|Default|GetShouldCache)
    (if (>= (Utilities|Array|Length (Variables|Default|GetInputCache)) (Variables|Default|GetInputCacheHistoryMaxNumber))
      (Utilities|Array|RemoveIndex (Variables|Default|GetInputCache)))
    (Utilities|Array|Add (Variables|Default|GetInputCache) NewInput)))

(fn GetInputCache
  (if (<= (Utilities|Array|Length (Variables|Default|GetInputCache)) 0)
    (return "NewEnumerator6")
    (else
      (return (Utilities|Array|Get(acopy) (Variables|Default|GetInputCache) (- (Utilities|Array|Length (Variables|Default|GetInputCache)) 1))))))

(fn CleanupInputCache
  (Utilities|Array|Clear (Variables|Default|GetInputCache)))